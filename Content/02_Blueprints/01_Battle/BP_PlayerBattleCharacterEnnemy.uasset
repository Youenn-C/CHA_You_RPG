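; Battle character Blueprint, named as an enemy variant, that tracks HP and drives its own battle UI widget.
; BeginPlay casts the widget component's content to BP_CharacterBattleUI and caches it.
; AddHP feeds ChangeHP, which stores HP, sends the HP/HPMax ratio to the UI and calls OnDeath at zero or below.
; OnDeath only prints a debug message, and Attack is an empty stub.
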(event EventBeginPlay
  (|CallParentFunction)
  (bind _asbp_character_battle_ui (Utilities|Casting|CastToBP_CharacterBattleUI (UserInterface|GetWidget (Variables|Default|GetWidget))))
  (Variables|Default|SetCharacterBattleUI _asbp_character_battle_ui))

(fn ConstructionScript
  (|CallParentFunction))

(fn ChangeHP
  (params (HP :type Float%20%28double-precision%29))
  (bind _output_get (Variables|Default|SetHP HP))
  (Default|UpdateHP (Variables|Default|GetCharacterBattleUI) (/ _output_get (Variables|Default|GetHP_Max)))
  (if (<= (Variables|Default|GetHP) 0.0)
    (CallFunction|OnDeath)))

(fn AddHP
  (params (B :type Float%20%28double-precision%29))
  (CallFunction|ChangeHP (+ (Variables|Default|GetHP) B)))

(fn OnDeath
  (Development|PrintString "I'm Dead"))

(fn Attack)